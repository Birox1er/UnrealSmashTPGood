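; Energy ball projectile for the Jamnes character that launches upward with a physics impulse on spawn and can explode.
; OnExplode clears CanMove, stops physics, enlarges the sphere and enables its overlaps for a brief window before destroying the actor.
; Sphere overlaps print the actor's name, then send any SmashCharacter other than the Ness reference damage and a scaled ejection vector with clamped vertical component.
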(event `self.ReceiveBeginPlay`
  (`PrimitiveComponent.AddImpulse` (`self.Sphere`) (0.0 0.0 750.0) "None" true))

(event `self.OnExplode`
  (bind _sphere (`self.Sphere`))
  (set `self.CanMove` false)
  (`PrimitiveComponent.SetSimulatePhysics` _sphere false)
  (set `PrimitiveComponent.bGenerateOverlapEvents` true _sphere)
  (`SceneComponent.SetRelativeScale3D` _sphere (4.0 4.0 4.0))
  (`KismetSystemLibrary.Delay` 0.3)
  (`self.K2_DestroyActor`))

(event `self.Sphere.OnComponentBeginOverlap`
  (params (OverlappedComponent :type "PrimitiveComponent Object Reference") (OtherActor :type "Actor Object Reference") (OtherComp :type "PrimitiveComponent Object Reference") (OtherBodyIndex :type Integer) (bFromSweep :type Boolean) (SweepResult :type "HitResult Structure (by ref)"))
  (bind (_returnvalue_x _returnvalue_y _returnvalue_z) (`KismetMathLibrary.BreakVector` (* (`KismetMathLibrary.Normal` (- (`self.K2_GetActorLocation`) (`self.K2_GetActorLocation`))) (`self.ExpulsionValue`))))
  (`KismetSystemLibrary.PrintString` (`KismetSystemLibrary.GetDisplayName` OtherActor))
  (if (!= (`self.Ness`) OtherActor)
    (bind _assmash_character (cast `SmashCharacter` OtherActor))
    (`SmashCharacter.OnDamageTaken` _assmash_character (`KismetMathLibrary.MakeVector` _returnvalue_x _returnvalue_y (`KismetMathLibrary.FClamp` _returnvalue_z 50.0 1000.0)) (`self.Damage`))))

(fn `UserConstructionScript`)